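; BP_Schrodinger is an interactable 3D item that duplicates itself whenever the player picks it up.
; Interacting toggles a held state and, on pickup, spawns another BP_Schrodinger at the object's location.
; Tick holds the object in front of player 0's camera with physics off and its widget shown, restoring physics and hiding the widget on release.
; Focus toggles custom depth rendering; the description toggle is set but never read here.
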(event Custom|InteractOnServer
  (Variables|Default|SetInteractToggle (not (Variables|Default|GetInteractToggle))))

(event Custom|DescriptionOnServer
  (Variables|Default|SetDescriptionToggle (not (Variables|Default|GetDescriptionToggle))))

(event EventTick
  (params (DeltaSeconds :type Float%20%28single-precision%29))
  (bind _returnvalue (Game|GetPlayerCameraManager 0))
  (bind _widget (Variables|Default|GetWidget))
  (bind _object (Variables|Default|Getobject))
  (if (Variables|Default|GetInteractToggle)
    (Physics|SetSimulatePhysics _object false)
    (Transformation|SetWorldLocation (Variables|Default|Getobject) (+ (Transformation|GetActorLocation _returnvalue) (* (Math|Vector|GetForwardVector (Transformation|GetActorRotation _returnvalue)) (Variables|Default|GetLength))) false false)
    (Rendering|SetVisibility _widget true false)
    (else
      (Physics|SetSimulatePhysics _object true)
      (Rendering|SetVisibility _widget false false))))

(event Collision|EventActorBeginOverlap
  (params (OtherActor :type Actor%20Object%20Reference)))

(event EventInterfaceToggleFocus
  (params (Focus :type Boolean))
  (Rendering|SetRenderCustomDepth (Variables|Default|Getobject) Focus))

(event EventInterfaceInteract
  (CallFunction|InteractonServer)
  (if (Variables|Default|GetInteractToggle)
    (Game|SpawnActorfromClass "BP_Schrodinger_C" (Math|Conversions|ToTransform(Vector) (Transformation|GetWorldLocation (Variables|Default|Getobject))) "AdjustIfPossibleButAlwaysSpawn" 0 0)))

(event EventBeginPlay)

(fn ConstructionScript)

(fn GetInteractionWidget
  (return 0))